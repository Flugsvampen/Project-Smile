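; Behavior tree node that keeps the SeenHiding blackboard flag updated for AI that detects a player hiding.
; On activation it caches the AI_Character_test pawn from the SelfActor blackboard key.
; Each tick it compares the character's PlayerSeenHiding with SeenHiding and, when they differ, writes IsPlayerVisible to that key rather than the compared value.
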(event `self.ReceiveActivation`
  (params (OwnerActor :type "Actor Object Reference"))
  (bind _asai_character_test (cast `/Game/Blueprints/AI/AI_Character_test` (`BTFunctionLibrary.GetBlackboardValueAsObject` (`self.SelfActor`))))
  (set `self.AI_Character` _asai_character_test))

(event `self.ReceiveTick`
  (params (OwnerActor :type "Actor Object Reference") (DeltaSeconds :type "Float (single-precision)"))
  (if (!= (`/Game/Blueprints/AI/AI_Character_test.PlayerSeenHiding` (`self.AI_Character`)) (`BTFunctionLibrary.GetBlackboardValueAsBool` (`self.SeenHiding`)))
    (`BTFunctionLibrary.SetBlackboardValueAsBool` (`self.SeenHiding`) (`/Game/Blueprints/AI/AI_Character_test.IsPlayerVisible` (`self.AI_Character`)))))