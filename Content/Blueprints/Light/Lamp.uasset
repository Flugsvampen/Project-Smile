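; Interactable lamp that, while lit, turns attached nav modifier volumes into NavArea_Null, blocking AI navigation.
; The null area is applied only when no AI_Character_test is inside the collision sphere, resizable to the light radius, and cleared on switch-off.
; A timer climbs while lit; at its limit a timeline flickers the light, then switches it off and locks interaction until the timer drains to zero.
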(event `self.ReceiveBeginPlay`
  (`self.SwitchOff`))

(event `StopBlinking`
  (`Timeline|Timeline_0` :!via `Stop` :!label _label
    (:`Finished`
      (`self.SwitchOff`)
      (set `self.CanSwitch` false))
    (:`LightSwitching`
      (`/Engine/EditorBlueprintResources/StandardMacros.FlipFlop`
        (:`A`
          (`SceneComponent.SetVisibility` (`self.PointLight`) true false))
        (:`B`
          (`SceneComponent.SetVisibility` (`self.PointLight`) false false))))))

(event `self.ReceiveTick`
  (params (DeltaSeconds :type "Float (single-precision)"))
  (if (and (`self.ShouldEnableNav`) (!= (`self.AiIsWithin`) true))
    (for _array_element (`self.GetAttachedActors`)
      (bind _asnav_modifier_volume (cast `NavModifierVolume` _array_element))
      (`NavModifierVolume.SetAreaClass` _asnav_modifier_volume "/Script/Engine.NavArea_Null")))
  (if (`self.Lit`)
    (set `self.LitTimer` (`KismetMathLibrary.FClamp` (+ (`self.LitTimer`) DeltaSeconds) 0.0 (`self.LitTimeLimit`)))
    (if (and (>= (`self.LitTimer`) (`self.LitTimeLimit`)) (!= (`self.IsAutoSwitching`) true))
      (set `self.IsAutoSwitching` true)
      (goto _label :!via `PlayFromStart`))
    (else
      (set `self.LitTimer` (`KismetMathLibrary.FClamp` (- (`self.LitTimer`) DeltaSeconds) 0.0 (`self.LitTimeLimit`)))
      (if (<= (`self.LitTimer`) 0.0)
        (set `self.CanSwitch` true)))))

(event `ResizeCollision`
  (`SphereComponent.SetSphereRadius` (`self.Collision`) (`PointLightComponent.AttenuationRadius` (`self.PointLight`)) true))

(event `Interact`
  (if (`self.CanSwitch`)
    (if (`self.Lit`)
      (`self.SwitchOff`)
      (else
        (`self.SwitchOn`)))))

(event `self.Collision.OnComponentBeginOverlap`
  (params (OverlappedComponent :type "PrimitiveComponent Object Reference") (OtherActor :type "Actor Object Reference") (OtherComp :type "PrimitiveComponent Object Reference") (OtherBodyIndex :type Integer) (bFromSweep :type Boolean) (SweepResult :type "HitResult Structure (by ref)"))
  (cast `/Game/Blueprints/AI/AI_Character_test` OtherActor)
  (set `self.AiIsWithin` true))

(event `self.Collision.OnComponentEndOverlap`
  (params (OverlappedComponent :type "PrimitiveComponent Object Reference") (OtherActor :type "Actor Object Reference") (OtherComp :type "PrimitiveComponent Object Reference") (OtherBodyIndex :type Integer))
  (cast `/Game/Blueprints/AI/AI_Character_test` OtherActor)
  (set `self.AiIsWithin` false))

(fn `InteractionAvailableObject`
  (returns (NewHandSymbol :type "/Game/Blueprints/UI/InteractionImageEnum Enum"))
  (return "NewEnumerator3"))

(fn `InteractWithObject`
  (params (Activator :type "Actor Object Reference"))
  (returns (Success :type Boolean))
  (`self.Interact`)
  (return false))

(fn `SwitchOff`
  (for _array_element (`self.GetAttachedActors`)
    (bind _asnav_modifier_volume (cast `NavModifierVolume` _array_element))
    (`NavModifierVolume.SetAreaClass` _asnav_modifier_volume null))
  (`SceneComponent.SetVisibility` (`self.PointLight`) false false)
  (set `self.Lit` false)
  (set `self.IsAutoSwitching` false)
  (set `self.ShouldEnableNav` false)
  (`self.StopBlinking`))

(fn `SwitchOn`
  (`SceneComponent.SetVisibility` (`self.PointLight`) true false)
  (set `self.Lit` true)
  (set `self.ShouldEnableNav` true))

(fn `UserConstructionScript`)