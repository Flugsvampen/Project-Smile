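; Bed is a hiding spot Blueprint that an AI character can search for a hidden player.
; Its Search event calls the parent logic, then checks ContainsPlayer to choose the AI's bed-specific response.
; If the player is inside, it calls BedSearchFound on the AI and clears the flag; otherwise it calls BedSearch.
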(event `self.Search`
  (params (`AI Character` :type "/Game/Blueprints/AI/AI_Character_test Object Reference"))
  (bind _ai_character (`self.AI Character`))
  (`parent.Search` `AI Character`)
  (if (`self.ContainsPlayer`)
    (`/Game/Blueprints/AI/AI_Character_test.BedSearch_found` _ai_character)
    (set `self.ContainsPlayer` false)
    (else
      (`/Game/Blueprints/AI/AI_Character_test.BedSearch` _ai_character))))

(fn `UserConstructionScript`
  (`parent.UserConstructionScript`))