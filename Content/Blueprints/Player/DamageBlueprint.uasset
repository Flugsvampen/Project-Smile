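; Damage actor that hurts the player character, MyCharacter, whenever it begins overlapping this actor.
; Each overlap subtracts the character's own HealthDecreaseAmount from its CurrentHealth, so the damage value lives on the character.
; At zero health or below it prints a death message and destroys the character; otherwise it prints the damage amount.
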(event `self.ReceiveActorBeginOverlap`
  (params (OtherActor :type "Actor Object Reference"))
  (bind _asmy_character (cast `/Game/Blueprints/Player/MyCharacter` OtherActor))
  (bind _healthdecreaseamount (`/Game/Blueprints/Player/MyCharacter.HealthDecreaseAmount` _asmy_character))
  (bind _output_get (set `/Game/Blueprints/Player/MyCharacter.CurrentHealth` (- (`/Game/Blueprints/Player/MyCharacter.CurrentHealth` _asmy_character) _healthdecreaseamount) _asmy_character))
  (if (<= _output_get 0.0)
    (`KismetSystemLibrary.PrintString` "You Died")
    (bind _asmy_character_2 (cast `/Game/Blueprints/Player/MyCharacter` OtherActor))
    (`self.K2_DestroyActor` _asmy_character_2)
    (else
      (`KismetSystemLibrary.PrintString` (`KismetStringLibrary.Conv_DoubleToString` _healthdecreaseamount)))))

(fn `UserConstructionScript`)