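; Base pickup actor that other objects can interact with, disappearing from the world once used.
; The construction script applies an optional replacement mesh and sets it to query-only overlap on a custom collision channel.
; Interaction reports a fixed availability type and deactivates the pickup through SetPickupActive, which toggles collision and visibility.
; SetPickupActive is kept separate because it also runs when a game is loaded.
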(fn `InteractionAvailableObject`
  (returns (NewHandSymbol :type "/Game/Blueprints/UI/InteractionImageEnum Enum"))
  (return "NewEnumerator1"))

(fn `InteractWithObject`
  (params (Activator :type "Actor Object Reference"))
  (returns (Success :type Boolean))
  ;[1 1 1] This is two separate function because the first one is called when game is loaded aswell
  (`self.SetPickupActive` false)
  (return true))

(fn `SetPickupActive`
  (params (IsActive :type Boolean))
  (`self.SetActorEnableCollision` IsActive)
  (`self.SetActorHiddenInGame` (not IsActive))
  (return))

(fn `UserConstructionScript`
  (bind _pickupablemesh (`self.PickupAbleMesh`))
  (bind _newmesh (`self.NewMesh`))
  ;[1 1 1] Comment
  (if (!= _newmesh null)
    (`StaticMeshComponent.SetStaticMesh` (`self.PickupAbleMesh`) _newmesh)
    (`PrimitiveComponent.SetCollisionObjectType` _pickupablemesh "ECC_GameTraceChannel1")
    (`PrimitiveComponent.SetCollisionResponseToAllChannels` _pickupablemesh "ECR_Overlap")
    (`PrimitiveComponent.SetCollisionEnabled` _pickupablemesh "QueryOnly")))