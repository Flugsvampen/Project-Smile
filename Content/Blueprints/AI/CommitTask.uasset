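; Behavior tree task that makes the AI character act on the path node it has reached, read from the DesiredPathNode blackboard key.
; For a SearchNode, it turns the character to each stored yaw through a custom for-each macro that delays between iterations, then finishes successfully.
; For a RoomNode, it simply waits briefly before finishing.
; Failed casts have no fallback, so other node types never finish the task.
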(event `self.ReceiveExecute`
  (params (OwnerActor :type "Actor Object Reference"))
  (bind _asai_character_test (cast `/Game/Blueprints/AI/AI_Character_test` (`BTFunctionLibrary.GetBlackboardValueAsActor` (`self.SelfActor`))))
  (set `self.AI` _asai_character_test)
  (`|ExecutionSequence`
    (:`then_0`
      ;[1 1 1] Rotates Z-axis of AI Character to angles stored in reached SearchNode
      (bind _assearch_node (cast `/Game/Blueprints/AI/SearchNode` (`BTFunctionLibrary.GetBlackboardValueAsObject` (`self.DesiredPathNode`))))
      (bind _arrayelement (`self.ForEachLoop_Delay` (`/Game/Blueprints/AI/SearchNode.Rotations` _assearch_node) 2.0)
        (:`LoopBody`
          (`self.CallRotateToRotation` 0.0 0.0 _arrayelement))
        (:`Completed`
          (`self.FinishExecute` true))))
    (:`then_1`
      ;[1 1 1] Waits when RoomNode is reached
      (cast `/Game/Blueprints/AI/RoomNode` (`BTFunctionLibrary.GetBlackboardValueAsObject` (`self.DesiredPathNode`)))
      (`KismetSystemLibrary.Delay` 2.0)
      (`self.FinishExecute` true))))

(fn `CallRotateToRotation`
  (params (X :type "Float (double-precision)") (Y :type "Float (double-precision)") (Z :type "Float (double-precision)"))
  (`/Game/Blueprints/AI/AI_Character_test.RotateToRotation` (`self.AI`) (`KismetMathLibrary.MakeRotator` X Y Z) 0.0))