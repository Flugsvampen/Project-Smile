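; Game instance Blueprint that tracks collectible page pickups and persists them in a PageSaveGame slot.
; PickupPage marks the page unlocked, saves at once, then pauses the game and shows a reusable PageDisplay widget with UI-only input.
; Saving creates the save object if none exists and writes the whole unlock array.
; Loading only merges true values, so collected pages are never re-locked.
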(fn `LoadPageArray`
  (bind _returnvalue (`GameplayStatics.LoadGameFromSlot` (`self.PageSaveName`)))
  (`/Engine/EditorBlueprintResources/StandardMacros.IsValid` _returnvalue
    (:`Is Valid`
      (bind _aspage_save_game (cast `/Game/Blueprints/Checkpoint/PageSaveGame` _returnvalue))
      ;[1 1 1] Pages stay picked up, wont change a value to false
      (for (_array_element _array_index) (`/Game/Blueprints/Checkpoint/PageSaveGame.UnlockTextArray` _aspage_save_game)
        (if _array_element
          (`KismetArrayLibrary.Array_Set` (`self.UnlockPageArray`) _array_index true))))
    (:`Is Not Valid`
      (`KismetSystemLibrary.PrintString` "Load pages failed")
      (return))))

(fn `PickupPage`
  (params (NewParam :type Integer))
  (bind _returnvalue (`GameplayStatics.GetPlayerController` 0))
  (bind _pagedisplayreference (`self.PageDisplayReference`))
  (`KismetArrayLibrary.Array_Set` (`self.UnlockPageArray`) NewParam true) ; No check as the variable is saved
  (`self.SavePageArray`) ; Saves the pages as they are picked up
  (`/Engine/EditorBlueprintResources/StandardMacros.IsValid` (`self.PageDisplayReference`)
    (:`Is Valid`
      _)
    (:`Is Not Valid`
      (bind _returnvalue_2 (`|CreateWidget` "/Game/Blueprints/UI/PageDisplay.PageDisplay_C" _returnvalue))
      (set `self.PageDisplayReference` _returnvalue_2)))
  (`/Game/Blueprints/UI/PageDisplay.SetPagesPickedUp` _pagedisplayreference (`self.UnlockPageArray`))
  (set `/Game/Blueprints/UI/PageDisplay.PageNr` NewParam _pagedisplayreference)
  (`WidgetBlueprintLibrary.SetInputMode_UIOnlyEx` _returnvalue _pagedisplayreference)
  (`GameplayStatics.SetGamePaused` true)
  (`UserWidget.AddToViewport` _pagedisplayreference 0)
  (set `PlayerController.bShowMouseCursor` true _returnvalue))

(fn `SavePageArray`
  (locals (LocalPageSaveGame :type "/Game/Blueprints/Checkpoint/PageSaveGame Object Reference"))
  (bind _localpagesavegame (`local.LocalPageSaveGame`))
  (bind _returnvalue (`GameplayStatics.DoesSaveGameExist` (`self.PageSaveName`)))
  (if _returnvalue
    (bind _returnvalue_2 (`GameplayStatics.LoadGameFromSlot` (`self.PageSaveName`)))
    (bind _aspage_save_game (cast `/Game/Blueprints/Checkpoint/PageSaveGame` _returnvalue_2))
    (set `local.LocalPageSaveGame` _aspage_save_game)
    (else
      (bind _returnvalue_3 (`GameplayStatics.CreateSaveGameObject` "/Game/Blueprints/Checkpoint/PageSaveGame.PageSaveGame_C"))
      (set `local.LocalPageSaveGame` _returnvalue_3)))
  (set `/Game/Blueprints/Checkpoint/PageSaveGame.UnlockTextArray` (`self.UnlockPageArray`) _localpagesavegame)
  (`GameplayStatics.SaveGameToSlot` _localpagesavegame (`self.PageSaveName`)))