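; HidingSpot is an interactable actor where the player can hide and AI characters can search.
; Interacting sends the player to the spot via its child-actor node, provided it is neither occupied nor flagged as searched.
; Search sets that flag, then either records this spot type as the AI's preference and plays a sound if the player is inside, or raises failed searches and lowers suspicion.
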(event `Search`
  (params (`AI Character` :type "/Game/Blueprints/AI/AI_Character_test Object Reference"))
  (set `self.AI Character` `AI Character`)
  (set `self.BeingSearched` true)
  (if (`self.ContainsPlayer`)
    (`/Game/Blueprints/AI/AI_Character_test.SetPreferredHidingSpot` (`self.AI Character`) (`self.HidingSpotType`))
    (`GameplayStatics.PlaySoundAtLocation` "/Game/Audio/VoiceActing/Cues/FailedSearch.FailedSearch" (`self.K2_GetActorLocation` (`self.AI Character`)))
    (else
      (`/Game/Blueprints/AI/AI_Character_test.IncreaseFailedSearches` (`self.AI Character`))
      (`/Game/Blueprints/AI/AI_Character_test.DecreaseSuspiciousness` (`self.AI Character`)))))

(event `Interact`
  (params (Player :type "/Game/Blueprints/Player/MyCharacter Object Reference"))
  (if (`self.BeingSearched`)
    _
    (elif (not (`self.ContainsPlayer`))
      (bind _output_get (set `self.Player` Player))
      (set `/Game/Blueprints/Player/MyCharacter.CurrentHidingSpot` self _output_get)
      (`/Game/Blueprints/Player/MyCharacter.GetToHidingSpot` _output_get (`self.K2_GetActorLocation` (`ChildActorComponent.ChildActor` (`self.HidingSpotNode`))) (`self.K2_GetActorLocation`)))))

(fn `InteractionAvailableObject`
  (returns (NewHandSymbol :type "/Game/Blueprints/UI/InteractionImageEnum Enum"))
  (return "NewEnumerator0"))

(fn `InteractWithObject`
  (params (Activator :type "Actor Object Reference"))
  (returns (Success :type Boolean))
  (bind _asmy_character (cast `/Game/Blueprints/Player/MyCharacter` Activator))
  (`self.Interact` _asmy_character)
  (return false))

(fn `UserConstructionScript`)