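; Enemy AI character that hunts the player, searches beds and shelves for hiding spots, attacks and performs a finishing kill.
; PawnSensing sight starts a sprint chase; losing sight for three seconds or hearing noise spawns an investigate node in the Blackboard.
; Timelines animate searches, pull-outs and attacks, toggling a damage box that drains health.
; It also tracks lamp and flashlight overlaps, failed searches and suspicion for its behavior logic.
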(event `self.ReceiveBeginPlay`
  (`KismetSystemLibrary.Delay` 1.0)
  (set `self.Blackboard` (`AIController.Blackboard` (`AIBlueprintHelperLibrary.GetAIController` self)))
  (set `CharacterMovementComponent.MaxWalkSpeed` (`self.WalkSpeed`) (`self.CharacterMovement`))
  (set `self.MinLightResistance` (`self.LightResistance`))
  (`PrimitiveComponent.SetCollisionResponseToAllChannels` (`self.Damage Box`) "ECR_Ignore")
  (`BlackboardComponent.SetValueAsInt` (`self.Blackboard`) (`self.FailedSearchesLimit_key`) 5)
  (`BlackboardComponent.SetValueAsInt` (`self.Blackboard`) (`self.FailedSearches_key`) 0)
  (`BlackboardComponent.SetValueAsBool` (`self.Blackboard`) (`self.SeenHiding`) false)
  (`BlackboardComponent.SetValueAsFloat` (`self.Blackboard`) (`self.LightResistace_key`) (`self.LightResistance`))
  (bind _outactors (`GameplayStatics.GetAllActorsWithTag` "Player"))
  (bind _asmy_character (cast `/Game/Blueprints/Player/MyCharacter` (`|GetArrayItem` _outactors)))
  (set `self.Player` _asmy_character))

(event `self.ReceiveHit`
  (params (MyComp :type "PrimitiveComponent Object Reference") (Other :type "Actor Object Reference") (OtherComp :type "PrimitiveComponent Object Reference") (bSelfMoved :type Boolean) (HitLocation :type "Vector Structure") (HitNormal :type "Vector Structure") (NormalImpulse :type "Vector Structure") (Hit :type "HitResult Structure (by ref)"))
  (bind _asmy_character (cast `/Game/Blueprints/Player/MyCharacter` Other))
  (set `self.Player` _asmy_character)
  (`BlackboardComponent.SetValueAsObject` (`self.Blackboard`) (`self.PlayerName_key`) (`self.Player`))
  (set `self.IsPlayerVisible` true)
  (`ActorComponent.Activate` (`self.ChaseSound`) false))

(event `self.CapsuleComponent.OnComponentBeginOverlap`
  (params (OverlappedComponent :type "PrimitiveComponent Object Reference") (OtherActor :type "Actor Object Reference") (OtherComp :type "PrimitiveComponent Object Reference") (OtherBodyIndex :type Integer) (bFromSweep :type Boolean) (SweepResult :type "HitResult Structure (by ref)"))
  (if (`self.ActorHasTag` OtherActor "Light")
    (bind _aslamp (cast `/Game/Blueprints/Light/Lamp` OtherActor)
      (:`then`
        (set `self.HitLamp` _aslamp)
        (set `self.WithinLamp` true))
      (:`CastFailed`
        (cast `/Game/Blueprints/FlashLightColl` OtherActor)
        (set `self.WithinLight` true)))))

(event `self.CapsuleComponent.OnComponentEndOverlap`
  (params (OverlappedComponent :type "PrimitiveComponent Object Reference") (OtherActor :type "Actor Object Reference") (OtherComp :type "PrimitiveComponent Object Reference") (OtherBodyIndex :type Integer))
  (cast `/Game/Blueprints/Light/Lamp` OtherActor
    (:`then`
      (`BlackboardComponent.SetValueAsBool` (`self.Blackboard`) (`self.HitByLamp`) false)
      (set `self.WithinLamp` false))
    (:`CastFailed`
      (cast `/Game/Blueprints/FlashLightColl` OtherActor)
      (`BlackboardComponent.SetValueAsBool` (`self.Blackboard`) (`self.HitByLight`) false)
      (set `self.WithinLight` false))))

(event `RotateToRotation`
  (params (Angles :type "Rotator Structure") (Speed :type "Float (double-precision)"))
  ;[1 1 1] Lerps Actor Rotation towards given rotation
  (bind (_direction _newtrack_0) (`Timeline|LookRotation_tl` :!via `PlayFromStart`)
    (:`Update`
      (if (not (or (`BlackboardComponent.GetValueAsBool` (`self.Blackboard`) (`self.IsPlayerVisible_key`)) (`BlackboardComponent.GetValueAsBool` (`self.Blackboard`) (`self.IsNoiseHeard_key`))))
        (`self.K2_SetActorRotation` (`KismetMathLibrary.RLerp` (`self.K2_GetActorRotation`) Angles _newtrack_0 true))))))

(event `BedSearch`
  (params (HidingSpot :type "/Game/Blueprints/HidingSpots/HidingSpot Object Reference"))
  (bind (_direction _rotx _posz) (`Timeline|BedSearchAnim_tl` :!via `PlayFromStart`)
    (:`Update`
      (`|ExecutionSequence`
        (:`then_0`
          (`SceneComponent.K2_SetRelativeRotation` (`self.Mesh`) (`KismetMathLibrary.MakeRotator` _rotx) false false))
        (:`then_1`
          (`SceneComponent.K2_SetRelativeLocation` (`self.Mesh`) (`KismetMathLibrary.MakeVector` 0.0 0.0 _posz) false false))))
    (:`Finished`
      (set `/Game/Blueprints/HidingSpots/HidingSpot.BeingSearched` false HidingSpot))))

(event `ResetDoOnce_foundLine`
  (goto _label :!via `Reset`))

(event `self.PawnSensing.OnSeePawn`
  (params (Pawn :type "Pawn Object Reference"))
  (bind _player (`self.Player`))
  ;[1 1 1] Initiates hunt of player if it is seen
  (if (not (`self.IsStunned`))
    (bind _asmy_character (cast `/Game/Blueprints/Player/MyCharacter` Pawn))
    (set `self.Player` _asmy_character)
    (`BlackboardComponent.SetValueAsObject` (`self.Blackboard`) (`self.PlayerName_key`) _player)
    (if (!= (`/Game/Blueprints/Player/MyCharacter.Hidden` _player) true)
      (set `self.IsPlayerVisible` true)
      (if (`/Game/Blueprints/Player/MyCharacter.EnteringHidingSpot` (`self.Player`))
        (set `self.PlayerSeenHiding` true)
        (`BlackboardComponent.SetValueAsObject` (`self.Blackboard`) (`self.DesiredPathNode_key`) (`ChildActorComponent.ChildActor` (`/Game/Blueprints/HidingSpots/HidingSpot.HidingSpotNode` (`/Game/Blueprints/Player/MyCharacter.CurrentHidingSpot` (`self.Player`))))))
      (set `CharacterMovementComponent.MaxWalkSpeed` (`self.SprintSpeed`) (`self.CharacterMovement`))
      (set `self.LastSeenPos` (`self.K2_GetActorLocation` (`self.Player`)))
      (`ActorComponent.Activate` (`self.ChaseSound`) false)
      (`|ExecutionSequence`
        (:`then_0`
          (`/Engine/EditorBlueprintResources/StandardMacros.DoOnce` false :!label _label
            (:`Completed`
              (`GameplayStatics.PlaySoundAtLocation` "/Game/Audio/VoiceActing/Cues/FoundPlayer.FoundPlayer" (`self.K2_GetActorLocation`)))))
        (:`then_1`
          ;[1 1 1] Player is lost when AI hasn't seen it in 3 seconds
          (`KismetSystemLibrary.RetriggerableDelay` 3.0)
          (if (not (`self.PlayerSeenHiding`))
            (set `self.IsPlayerVisible` false)
            (set `CharacterMovementComponent.MaxWalkSpeed` (`self.WalkSpeed`) (`self.CharacterMovement`))
            (`self.CreateInvestigateNode` (`self.LastSeenPos`))
            (`ActorComponent.Deactivate` (`self.ChaseSound`))
            (`self.ResetDoOnce_foundLine`)))))))

(event `self.PawnSensing.OnHearNoise`
  (params (Instigator :type "Pawn Object Reference") (Location :type "Vector Structure (by ref)") (Volume :type "Float (single-precision)"))
  ;[1 1 1] Noise Hearing
  (if (not (`self.IsPlayerVisible`))
    (set `self.NoiseHeard` true)
    (`self.CreateInvestigateNode` Location)))

(event `BedSearch_found`
  (params (NodeLocation :type "Vector Structure") (HidingSpot :type "/Game/Blueprints/HidingSpots/HidingSpot Object Reference"))
  (bind (_direction _rotx _posz _posx) (`Timeline|Timeline_0` :!via `PlayFromStart`)
    (:`Update`
      (`|ExecutionSequence`
        (:`then_0`
          (`SceneComponent.K2_SetRelativeRotation` (`self.Mesh`) (`KismetMathLibrary.MakeRotator` _rotx) false false))
        (:`then_1`
          (`SceneComponent.K2_SetRelativeLocation` (`self.Mesh`) (`KismetMathLibrary.MakeVector` _posx 0.0 _posz) false false))))
    (:`Finished`
      (`PrimitiveComponent.SetCollisionResponseToAllChannels` (`self.Damage Box`) "ECR_Ignore"))
    (:`PullOut`
      (`/Game/Blueprints/Player/MyCharacter.ExitHiding_Lerp` (`self.Player`) NodeLocation)
      (set `/Game/Blueprints/HidingSpots/HidingSpot.BeingSearched` false HidingSpot)
      (set `self.IsPlayerVisible` true)
      (`PrimitiveComponent.SetCollisionResponseToAllChannels` (`self.Damage Box`) "ECR_Overlap"))))

(event `self.Damage Box.OnComponentBeginOverlap`
  (params (OverlappedComponent :type "PrimitiveComponent Object Reference") (OtherActor :type "Actor Object Reference") (OtherComp :type "PrimitiveComponent Object Reference") (OtherBodyIndex :type Integer) (bFromSweep :type Boolean) (SweepResult :type "HitResult Structure (by ref)"))
  ;[1 1 1] Decreases player health, and potentially kills it, when it is inside Damage Box
  (cast `CapsuleComponent` OtherComp)
  (bind _asmy_character (cast `/Game/Blueprints/Player/MyCharacter` OtherActor))
  (bind _output_get (set `/Game/Blueprints/Player/MyCharacter.CurrentHealth` (- (`/Game/Blueprints/Player/MyCharacter.CurrentHealth` _asmy_character) (`/Game/Blueprints/Player/MyCharacter.HealthDecreaseAmount` _asmy_character)) _asmy_character))
  (`/Game/Blueprints/Player/MyCharacter.UpdateHealth` _asmy_character _output_get)
  (if (<= _output_get 0.0)
    (`self.Finishing Blow` false)))

(event `Attack`
  (bind _damage_box (`self.Damage Box`))
  ;[1 1 1] Plays attack animation that also activates Damage Box
  (if (not (`self.IsFinishing`))
    (set `self.IsAttacking` true)
    (bind (_direction _rotation) (`Timeline|AttackAnim_tl` :!via `PlayFromStart`)
      (:`Finished`
        (set `self.IsAttacking` false))
      (:`Toggle Damage Box`
        (`/Engine/EditorBlueprintResources/StandardMacros.FlipFlop`
          (:`A`
            (`PrimitiveComponent.SetCollisionResponseToAllChannels` _damage_box "ECR_Overlap"))
          (:`B`
            (`PrimitiveComponent.SetCollisionResponseToAllChannels` _damage_box "ECR_Ignore")))))))

(event `ShelvesFound`
  (params (NodeLoacation :type "Vector Structure") (HidingSpot :type "/Game/Blueprints/HidingSpots/HidingSpot Object Reference"))
  (`Timeline|ShelvesFound_anim`
    (:`Finished`
      (`PrimitiveComponent.SetCollisionResponseToAllChannels` (`self.Damage Box`) "ECR_Ignore"))
    (:`PullOut`
      (`/Game/Blueprints/Player/MyCharacter.ExitHiding_Lerp` (`self.Player`) NodeLoacation)
      (set `/Game/Blueprints/HidingSpots/HidingSpot.BeingSearched` false HidingSpot)
      (set `self.IsPlayerVisible` true)
      (`PrimitiveComponent.SetCollisionResponseToAllChannels` (`self.Damage Box`) "ECR_Overlap"))))

(event `ShelvesSearch`
  (params (HidingSpot :type "/Game/Blueprints/HidingSpots/HidingSpot Object Reference"))
  (`Timeline|ShelvesSearch_anim`
    (:`Finished`
      (set `/Game/Blueprints/HidingSpots/HidingSpot.BeingSearched` false HidingSpot))))

(event `Finishing Blow`
  (params (Player :type Boolean))
  (bind _player (`self.Player`))
  (set `/Game/Blueprints/Player/MyCharacter.Killed` true _player)
  (`/Game/Blueprints/Player/MyCharacter.RotateTowards` _player (`self.K2_GetActorLocation`))
  (`GameplayStatics.PlaySoundAtLocation` "/Game/Audio/VoiceActing/Cues/KillPlayer.KillPlayer" (`self.K2_GetActorLocation`))
  (`SceneComponent.K2_SetRelativeRotation` :`self` (`self.Mesh`))
  (set `self.IsFinishing` true)
  (bind (_direction _xrot _xpos) (`Timeline|FinisherAnim_tl` :!via `PlayFromStart`)
    (:`KillPlayer`
      (`self.K2_DestroyActor` (`self.Player`))
      (set `self.IsFinishing` false))))

(fn `CreateInvestigateNode`
  (params (Location :type "Vector Structure"))
  (bind _returnvalue (`|SpawnActorFromClass` "/Game/Blueprints/AI/Nodes/InvestigateNode.InvestigateNode_C" (`KismetMathLibrary.Conv_VectorToTransform` Location) "Undefined" "OverrideRootScale" null null))
  (`BlackboardComponent.SetValueAsObject` (`self.Blackboard`) (`self.DesiredPathNode_key`) _returnvalue)
  (return))

(fn `DecreaseSuspiciousness`
  (`BlackboardComponent.SetValueAsInt` (`self.Blackboard`) (`self.Suspiciousness`) (- (`BlackboardComponent.GetValueAsInt` (`self.Blackboard`) (`self.Suspiciousness`)) 1)))

(fn `IncreaseFailedSearches`
  (bind _returnvalue (+ (`BlackboardComponent.GetValueAsInt` (`self.Blackboard`) (`self.FailedSearches_key`)) 1))
  (`BlackboardComponent.SetValueAsInt` (`self.Blackboard`) (`self.FailedSearches_key`) _returnvalue)
  (if (== _returnvalue (`BlackboardComponent.GetValueAsInt` (`self.Blackboard`) (`self.FailedSearchesLimit_key`)))
    (`self.SetPreferredHidingSpot` "NewEnumerator0")
    (`BlackboardComponent.SetValueAsInt` (`self.Blackboard`) (`self.FailedSearches_key`) 0)))

(fn `SetPreferredHidingSpot`
  (params (HidingSpotType :type "/Game/Blueprints/AI/HidingSpotTypes Enum" :default "NewEnumerator0"))
  (`BlackboardComponent.SetValueAsEnum` (`self.Blackboard`) (`self.PreferredHidingSpotType_key`) HidingSpotType)
  (`BlackboardComponent.SetValueAsInt` (`self.Blackboard`) (`self.FailedSearches_key`) 0))

(fn `UserConstructionScript`)