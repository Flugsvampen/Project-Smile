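; Collectible page pickup, a child of a pickupable base, that unlocks one page identified by its TextNumber.
; Interacting calls PickupPage on the PageGameInstance with that number, then runs the parent interaction.
; CheckPagePickedup reads the game instance's UnlockPageArray and deactivates the pickup if that page is already unlocked.
; InteractionAvailableObject reports a fixed enum value as its interaction availability.
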(fn `CheckPagePickedup`
  (bind _aspage_game_instance (cast `/Game/Blueprints/Checkpoint/PageGameInstance` (`GameplayStatics.GetGameInstance`)))
  (if (`|GetArrayItem` (`/Game/Blueprints/Checkpoint/PageGameInstance.UnlockPageArray` _aspage_game_instance) (`self.TextNumber`))
    (`self.SetPickupActive` false)))

(fn `InteractionAvailableObject`
  (returns (NewHandSymbol :type "/Game/Blueprints/UI/InteractionImageEnum Enum"))
  (return "NewEnumerator1"))

(fn `InteractWithObject`
  (params (Activator :type "Actor Object Reference"))
  (returns (Success :type Boolean))
  (bind _aspage_game_instance (cast `/Game/Blueprints/Checkpoint/PageGameInstance` (`GameplayStatics.GetGameInstance`)))
  (`/Game/Blueprints/Checkpoint/PageGameInstance.PickupPage` _aspage_game_instance (`self.TextNumber`))
  (bind _success (`parent.InteractWithObject` null))
  (return _success))

(fn `UserConstructionScript`
  (`parent.UserConstructionScript`))