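; Level actor that saves and loads progress in a single auto-save slot and tracks collectible text pages.
; SaveGame records player key and battery counts, pickup collision states, unlocked pages and door lock/rotation; LoadGame reapplies them by index to the object and door arrays.
; PickupPage unlocks a page and displays text, but only writes to disk when no save exists.
; Player overlap re-enables all pickups as a placeholder test.
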(event `self.ReceiveBeginPlay`)

(event `self.ReceiveActorBeginOverlap`
  (params (OtherActor :type "Actor Object Reference"))
  ;[1 1 1] Placeholder event, setindex should be called by load
  (if (== (`GameplayStatics.GetObjectClass` OtherActor) "/Game/Blueprints/Player/MyCharacter.MyCharacter_C")
    (`self.ResetStatusObjects`)))

(fn `GetPage`
  (params (PageId :type Integer))
  (returns (Text :type String) (Success :type Boolean))
  (if (`|GetArrayItem` (`self.UnlockPageArray`) PageId)
    (return (`|GetArrayItem` (`self.PageArray`) PageId) true)
    (else
      (return "" false))))

(fn `LoadGame`
  (bind _autosavegame (`self.AutoSaveGame`))
  (bind _returnvalue (`self.GetComponentByClass` (`GameplayStatics.GetPlayerCharacter` 0) "/Game/Blueprints/UI/Inventory.Inventory_C"))
  (bind _returnvalue_2 (`GameplayStatics.LoadGameFromSlot` (`self.AutoSaveName`)))
  (`/Engine/EditorBlueprintResources/StandardMacros.IsValid` _returnvalue_2
    (:`Is Valid`
      (bind _asmy_save_game (cast `/Game/Blueprints/Checkpoint/MySaveGame` _returnvalue_2))
      (bind _output_get (set `self.AutoSaveGame` _asmy_save_game))
      (set `/Game/Blueprints/UI/Inventory.NumberOfKeys` (`/Game/Blueprints/Checkpoint/MySaveGame.AmountOfKeys` _output_get) _returnvalue)
      (set `/Game/Blueprints/UI/Inventory.NumberOfBatteries` (`/Game/Blueprints/Checkpoint/MySaveGame.AmountOfBatteries` _output_get) _returnvalue)
      (bind _output_get_2 (set `self.ActiveStatusArray` (`/Game/Blueprints/Checkpoint/MySaveGame.ObjectActiveArray` _output_get)))
      (`self.SetStatusFromArray` _output_get_2)
      (for (_array_element _array_index) (`/Game/Blueprints/Checkpoint/MySaveGame.UnlockTextArr` _output_get)
        (if _array_element
          (`KismetArrayLibrary.Array_Set` (`self.UnlockPageArray`) _array_index true)))
      (for (_array_element_2 _array_index_2) (`self.DoorArray`)
        (`/Game/Blueprints/SM_DoorFrame.SetDoorStatus` _array_element_2 (`|GetArrayItem` (`/Game/Blueprints/Checkpoint/MySaveGame.DoorRotationArray` _autosavegame) _array_index_2) (`|GetArrayItem` (`/Game/Blueprints/Checkpoint/MySaveGame.DoorUnlockedArray` _autosavegame) _array_index_2))))
    (:`Is Not Valid`
      (`KismetSystemLibrary.PrintString` "Load fail"))))

(fn `PickupPage`
  (params (PageId :type Integer))
  (`KismetArrayLibrary.Array_Set` (`self.UnlockPageArray`) PageId true)
  (bind _asmy_character (cast `/Game/Blueprints/Player/MyCharacter` (`GameplayStatics.GetPlayerCharacter` 0)))
  (`/Game/Blueprints/UI/Inventory.DisplayText` (`/Game/Blueprints/Player/MyCharacter.Inventory` _asmy_character) (`|GetArrayItem` (`self.PageArray`)))
  (bind _returnvalue (`GameplayStatics.DoesSaveGameExist` (`self.AutoSaveName`)))
  (if _returnvalue
    ;[1 1 1] Merely updates the changes to the page to the savegame.
    (bind _returnvalue_2 (`GameplayStatics.LoadGameFromSlot` (`self.AutoSaveName`)))
    (bind _asmy_save_game (cast `/Game/Blueprints/Checkpoint/MySaveGame` _returnvalue_2))
    (set `self.AutoSaveGame` _asmy_save_game)
    (set `/Game/Blueprints/Checkpoint/MySaveGame.UnlockTextArr` (`self.UnlockPageArray`) (`self.AutoSaveGame`))
    (else
      ;[1 1 1] Complete save game
      (`self.SaveGame`))))

(fn `ResetStatusObjects`
  ;[1 1 1] Testing function, will reset the status of all existing objects
  (for _array_element (`self.ObjectsArray`)
    (`/Game/Blueprints/Pickupable/Pickups.SetPickupActive` _array_element true)))

(fn `SaveGame`
  (bind _autosavegame (`self.AutoSaveGame`))
  (bind _autosavegame_2 (`self.AutoSaveGame`))
  (bind _autosavegame_3 (`self.AutoSaveGame`))
  (bind _returnvalue (`self.GetComponentByClass` (`GameplayStatics.GetPlayerCharacter` 0) "/Game/Blueprints/UI/Inventory.Inventory_C"))
  (bind _returnvalue_2 (`GameplayStatics.DoesSaveGameExist` (`self.AutoSaveName`)))
  (if _returnvalue_2
    (bind _returnvalue_3 (`GameplayStatics.LoadGameFromSlot` (`self.AutoSaveName`)))
    (bind _asmy_save_game (cast `/Game/Blueprints/Checkpoint/MySaveGame` _returnvalue_3))
    (set `self.AutoSaveGame` _asmy_save_game)
    (else
      (bind _returnvalue_4 (`GameplayStatics.CreateSaveGameObject` "/Game/Blueprints/Checkpoint/MySaveGame.MySaveGame_C"))
      (set `self.AutoSaveGame` _returnvalue_4)))
  (set `/Game/Blueprints/Checkpoint/MySaveGame.AmountOfKeys` (`/Game/Blueprints/UI/Inventory.NumberOfKeys` _returnvalue) _autosavegame_2)
  (set `/Game/Blueprints/Checkpoint/MySaveGame.AmountOfBatteries` (`/Game/Blueprints/UI/Inventory.NumberOfBatteries` _returnvalue) _autosavegame_2)
  ;[1 1 1] Resets the array and reads the value from each of the objects used
  (`KismetArrayLibrary.Array_Clear` (`self.ActiveStatusArray`))
  (for _array_element (`self.ObjectsArray`)
    (`KismetArrayLibrary.Array_Add` (`self.ActiveStatusArray`) (`PrimitiveComponent.K2_IsCollisionEnabled` (`/Game/Blueprints/Pickupable/Pickups.PickupAbleMesh` _array_element))))
  (set `/Game/Blueprints/Checkpoint/MySaveGame.ObjectActiveArray` (`self.ActiveStatusArray`) _autosavegame_2)
  (set `/Game/Blueprints/Checkpoint/MySaveGame.UnlockTextArr` (`self.UnlockPageArray`) _autosavegame_2)
  (`KismetArrayLibrary.Array_Clear` (`/Game/Blueprints/Checkpoint/MySaveGame.DoorRotationArray` _autosavegame_3))
  (`KismetArrayLibrary.Array_Clear` (`/Game/Blueprints/Checkpoint/MySaveGame.DoorUnlockedArray` _autosavegame_3))
  (for _array_element_2 (`self.DoorArray`)
    (bind (_zrotation _islocked) (`/Game/Blueprints/SM_DoorFrame.GetDoorStatus` _array_element_2))
    (`KismetArrayLibrary.Array_Add` (`/Game/Blueprints/Checkpoint/MySaveGame.DoorUnlockedArray` _autosavegame) _islocked)
    (`KismetArrayLibrary.Array_Add` (`/Game/Blueprints/Checkpoint/MySaveGame.DoorRotationArray` _autosavegame) _zrotation))
  (`GameplayStatics.SaveGameToSlot` (`self.AutoSaveGame`) (`self.AutoSaveName`))
  (return))

(fn `SetStatusFromArray`
  (params (NewStatusArray :type "Array of Boolean"))
  (returns (LoadResult :type Boolean))
  (locals (NewLocalVar_0 :type Integer))
  (if (== (`KismetArrayLibrary.Array_Length` NewStatusArray) (`KismetArrayLibrary.Array_Length` (`self.ObjectsArray`)))
    (for (_array_element _array_index) (`self.ObjectsArray`)
      (`/Game/Blueprints/Pickupable/Pickups.SetPickupActive` _array_element (`|GetArrayItem` NewStatusArray _array_index))
      ;[1 1 1] If cast fails then it will be ignored
      (bind _aspage (cast `/Game/Blueprints/Pickupable/Page` _array_element))
      (`/Game/Blueprints/Pickupable/Page.CheckPagePickedup` _aspage (`self.UnlockPageArray`) self))
    (return true)
    (else
      (return false))))

(fn `UserConstructionScript`)