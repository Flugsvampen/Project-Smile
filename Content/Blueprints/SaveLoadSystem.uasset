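; Level actor that saves and loads the player's key count and tracks unlocked pages and pickup states.
; SaveGame and LoadGame move the Inventory key count through an auto-save slot; page and pickup arrays are not written to it.
; A placeholder player overlap either applies the status array to all PickupAble actors or, on length mismatch, rebuilds it, assigning IDs and back-links.
; PickupPage unlocks pages but always displays the first one.
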(event `self.ReceiveActorBeginOverlap`
  (params (OtherActor :type "Actor Object Reference"))
  ;[1 1 1] Placeholder event, setindex should be called by load
  (if (== (`GameplayStatics.GetObjectClass` OtherActor) "/Game/Blueprints/MyCharacter.MyCharacter_C")
    (`self.SetIndexPickupable` (`self.ActiveStatusArray`))))

(fn `GetPage`
  (params (PageId :type Integer))
  (returns (Text :type String) (Success :type Boolean))
  (if (`|GetArrayItem` (`self.UnlockPageArray`) PageId)
    (return (`|GetArrayItem` (`self.PageArray`) PageId) true)
    (else
      (return "" false))))

(fn `LoadGame`
  (bind _returnvalue (`GameplayStatics.LoadGameFromSlot` (`self.AutoSaveName`)))
  (`/Engine/EditorBlueprintResources/StandardMacros.IsValid` _returnvalue
    (:`Is Valid`
      (bind _asmy_save_game (cast `/Game/Blueprints/Checkpoint/MySaveGame` _returnvalue))
      (bind _output_get (set `self.AutoSaveGame` _asmy_save_game))
      (set `/Game/Blueprints/UI/Inventory.NumberOfKeys` (`/Game/Blueprints/Checkpoint/MySaveGame.AmountOfKeys` _output_get) (`self.GetComponentByClass` (`GameplayStatics.GetPlayerCharacter` 0) "/Game/Blueprints/UI/Inventory.Inventory_C")))
    (:`Is Not Valid`
      (`KismetSystemLibrary.PrintString` "Load fail"))))

(fn `ObjectDeactivated`
  (params (NewParam :type Integer))
  (`KismetArrayLibrary.Array_Set` (`self.ActiveStatusArray`) NewParam))

(fn `PickupPage`
  (params (PageId :type Integer) (ObjectID :type Integer))
  (`KismetArrayLibrary.Array_Set` (`self.ActiveStatusArray`) ObjectID)
  (`KismetArrayLibrary.Array_Set` (`self.UnlockPageArray`) PageId true)
  (bind _asmy_character (cast `/Game/Blueprints/MyCharacter` (`GameplayStatics.GetPlayerCharacter` 0)))
  (`/Game/Blueprints/UI/Inventory.DisplayText` (`/Game/Blueprints/MyCharacter.Inventory` _asmy_character) (`|GetArrayItem` (`self.PageArray`)))
  (return))

(fn `SaveGame`
  (bind _returnvalue (`GameplayStatics.DoesSaveGameExist` (`self.AutoSaveName`)))
  (if _returnvalue
    (bind _returnvalue_2 (`GameplayStatics.LoadGameFromSlot` (`self.AutoSaveName`)))
    (bind _asmy_save_game (cast `/Game/Blueprints/Checkpoint/MySaveGame` _returnvalue_2))
    (set `self.AutoSaveGame` _asmy_save_game)
    (else
      (bind _returnvalue_3 (`GameplayStatics.CreateSaveGameObject` "/Game/Blueprints/Checkpoint/MySaveGame.MySaveGame_C"))
      (set `self.AutoSaveGame` _returnvalue_3)))
  (set `/Game/Blueprints/Checkpoint/MySaveGame.AmountOfKeys` (`/Game/Blueprints/UI/Inventory.NumberOfKeys` (`self.GetComponentByClass` (`GameplayStatics.GetPlayerCharacter` 0) "/Game/Blueprints/UI/Inventory.Inventory_C")) (`self.AutoSaveGame`))
  (`GameplayStatics.SaveGameToSlot` (`self.AutoSaveGame`) (`self.AutoSaveName`)))

(fn `SetIndexPickupable`
  (params (NewStatusArray :type "Array of Boolean"))
  (locals (NewLocalVar_0 :type Integer))
  (bind _outactors (`GameplayStatics.GetAllActorsOfClass` "/Game/Blueprints/Pickupable/PickupAble.PickupAble_C"))
  (set `self.ObjectsArray` _outactors)
  (if (== (`KismetArrayLibrary.Array_Length` NewStatusArray) (`KismetArrayLibrary.Array_Length` _outactors))
    (for (_array_element _array_index) (`self.ObjectsArray`)
      (`/Game/Blueprints/Pickupable/PickupAble.SetPickupActive` _array_element (`|GetArrayItem` NewStatusArray _array_index)))
    (else
      ;[1 1 1] Builds the Active Status array to hold the status of all the pickupable objects in the level
      (`KismetArrayLibrary.Array_Clear` (`self.ActiveStatusArray`))
      (for _array_element_2 (`self.ObjectsArray`)
        (bind _returnvalue (`KismetArrayLibrary.Array_Add` (`self.ActiveStatusArray`) (`PrimitiveComponent.K2_IsCollisionEnabled` (`/Game/Blueprints/Pickupable/PickupAble.PickupAbleMesh` _array_element_2))))
        (set `/Game/Blueprints/Pickupable/PickupAble.Id` _returnvalue _array_element_2)
        (set `/Game/Blueprints/Pickupable/PickupAble.DeactivateLink` self _array_element_2))
      (`KismetSystemLibrary.PrintString` (`KismetStringLibrary.Conv_IntToString` (`KismetArrayLibrary.Array_Length` (`self.ActiveStatusArray`)))))))

(fn `UserConstructionScript`)