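; Health pickup actor that heals the player character when overlapped.
; On overlap it casts to MyCharacter and, if health is below maximum, adds the character's own HealthIncreaseAmount, prints a fixed +25HP message and destroys itself.
; At full health it only prints a Max Health message and stays in the world; the added health is not clamped to the maximum.
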(event `self.ReceiveActorBeginOverlap`
  (params (OtherActor :type "Actor Object Reference"))
  (bind _asmy_character (cast `/Game/Blueprints/MyCharacter` OtherActor))
  (if (< (`/Game/Blueprints/MyCharacter.CurrentHealth` _asmy_character) (`/Game/Blueprints/MyCharacter.MaxHealth` _asmy_character))
    (set `/Game/Blueprints/MyCharacter.CurrentHealth` (+ (`/Game/Blueprints/MyCharacter.CurrentHealth` _asmy_character) (`/Game/Blueprints/MyCharacter.HealthIncreaseAmount` _asmy_character)) _asmy_character)
    (`KismetSystemLibrary.PrintString` "+25HP")
    (`self.K2_DestroyActor`)
    (else
      (`KismetSystemLibrary.PrintString` "Max Health"))))

(fn `UserConstructionScript`)