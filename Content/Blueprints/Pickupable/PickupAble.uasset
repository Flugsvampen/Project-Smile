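; Base pickup actor Blueprint that provides a configurable mesh and stub interaction functions.
; SetPickupActive toggles visibility and collision together.
; The mesh-replacement function, marked mandatory in construction though the construction script here is empty, applies NewMesh with query-only overlap collision on a custom object channel.
; ActivateObject returns false and InteractionAvailableObject returns a fixed enum value, serving as defaults.
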(fn `ActivateObject`
  (params (Activator :type "Actor Object Reference"))
  (returns (Success :type Boolean))
  (return false))

(fn `InteractionAvailableObject`
  (returns (NewHandSymbol :type "/Game/Blueprints/UI/InteractionImageEnum Enum"))
  (return "NewEnumerator1"))

(fn `ReplaceMesh(mandatory in construction)`
  (bind _pickupablemesh (`self.PickupAbleMesh`))
  (bind _newmesh (`self.NewMesh`))
  ;[1 1 1] Comment
  (if (!= _newmesh null)
    (`StaticMeshComponent.SetStaticMesh` (`self.PickupAbleMesh`) _newmesh)
    (`PrimitiveComponent.SetCollisionObjectType` _pickupablemesh "ECC_GameTraceChannel1")
    (`PrimitiveComponent.SetCollisionResponseToAllChannels` _pickupablemesh "ECR_Overlap")
    (`PrimitiveComponent.SetCollisionEnabled` _pickupablemesh "QueryOnly")))

(fn `SetPickupActive`
  (params (IsActive :type Boolean))
  (`self.SetActorHiddenInGame` (not IsActive))
  (`self.SetActorEnableCollision` IsActive)
  (return))

(fn `UserConstructionScript`)