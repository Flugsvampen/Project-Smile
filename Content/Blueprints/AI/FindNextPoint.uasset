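; Behavior tree task that picks the AI character's next patrol point and stores it in the DesiredPathNode blackboard key.
; An unsearched RoomNode leads to its SearchNode and is marked searched, while a searched one advances to its NextNode and clears that node's Searched flag.
; A SearchNode simply passes to its NextNode.
; The AI then rotates on yaw toward the new point and the task finishes successfully.
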(event `self.ReceiveExecute`
  (params (OwnerActor :type "Actor Object Reference"))
  (bind _returnvalue (`BTFunctionLibrary.GetBlackboardValueAsObject` (`self.DesiredPathNode`)))
  (bind _asai_character_test (cast `/Game/Blueprints/AI/AI_Character_test` (`BTFunctionLibrary.GetBlackboardValueAsObject` (`self.SelfActor`))))
  (set `self.AI` _asai_character_test)
  (bind _asroom_node (cast `/Game/Blueprints/AI/RoomNode` _returnvalue)
    (:`then`
      (if (`/Game/Blueprints/AI/RoomNode.Searched` _asroom_node)
        (bind _nextnode (`/Game/Blueprints/AI/RoomNode.NextNode` _asroom_node))
        ;[1 1 1] Sets DesiredPathNode as NextNode(RoomNode) if this node already has been reached
        (`BTFunctionLibrary.SetBlackboardValueAsObject` (`self.DesiredPathNode`) _nextnode)
        (set `/Game/Blueprints/AI/RoomNode.Searched` false _nextnode)
        (else
          ;[1 1 1] Sets DesiredPathNode as SearchNode if this node hasn't been reached
          (`BTFunctionLibrary.SetBlackboardValueAsObject` (`self.DesiredPathNode`) (`/Game/Blueprints/AI/RoomNode.SearchNode` _asroom_node))
          (set `/Game/Blueprints/AI/RoomNode.Searched` true _asroom_node))))
    (:`CastFailed`
      (bind _assearch_node (cast `/Game/Blueprints/AI/SearchNode` _returnvalue))
      (`BTFunctionLibrary.SetBlackboardValueAsObject` (`self.DesiredPathNode`) (`/Game/Blueprints/AI/SearchNode.NextNode` _assearch_node))))
  ;[1 1 1] Rotates AI Character towards DesiredPathNode in Z-axis
  (`/Game/Blueprints/AI/AI_Character_test.RotateToRotation` (`self.AI`) (`KismetMathLibrary.MakeRotator` 0.0 0.0 (.yaw (`KismetMathLibrary.FindLookAtRotation` (`Actor.K2_GetActorLocation` (`self.AI`)) (`Actor.K2_GetActorLocation` (`BTFunctionLibrary.GetBlackboardValueAsActor` (`self.DesiredPathNode`)))))) 0.0)
  (`self.FinishExecute` true))